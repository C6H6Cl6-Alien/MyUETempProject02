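; Player controller that reads WASD keys and drives the possessed MyBaseCharacter's movement.
; Key press and release events set per-key flags, and BeginPlay caches player 0's pawn as the character.
; Every tick the flags resolve into forward/backward and right/left scales, where opposing keys cancel out.
; The resulting 2D vector is passed to the character's UpdateMovementState.
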(event `self.ReceiveBeginPlay`
  (bind _asmy_base_character (cast `/Game/Blueprints/MyBaseCharacter` (`GameplayStatics.GetPlayerPawn` 0)))
  (set `self.PlayerCharacter` _asmy_base_character))

(event `self.ReceiveTick`
  (params (DeltaSeconds :type "Float (single-precision)"))
  (`self.UpdateCharacterMovementState`))

(event `Key|W`
  (params (Key :type "Key Structure"))
  (:`Pressed`
    (set `self.KeyWPressing` true))
  (:`Released`
    (set `self.KeyWPressing` false)))

(event `Key|A`
  (params (Key :type "Key Structure"))
  (:`Pressed`
    (set `self.KeyAPressing` true))
  (:`Released`
    (set `self.KeyAPressing` false)))

(event `Key|S`
  (params (Key :type "Key Structure"))
  (:`Pressed`
    (set `self.KeySPressing` true))
  (:`Released`
    (set `self.KeySPressing` false)))

(event `Key|D`
  (params (Key :type "Key Structure"))
  (:`Pressed`
    (set `self.KeyDPressing` true))
  (:`Released`
    (set `self.KeyDPressing` false)))

(fn `UpdateCharacterMovementState`
  (locals (ForwardBackwardScale :type "Float (double-precision)") (RightLeftScale :type "Float (double-precision)"))
  (`|ExecutionSequence`
    (:`then_0`
      (if (and (`self.KeyWPressing`) (not (`self.KeySPressing`)))
        (set `local.ForwardBackwardScale` 1.0)
        (elif (and (not (`self.KeyWPressing`)) (`self.KeySPressing`))
          (set `local.ForwardBackwardScale` -1.0)
          (else
            (set `local.ForwardBackwardScale` 0.0)))))
    (:`then_1`
      (if (and (`self.KeyDPressing`) (not (`self.KeyAPressing`)))
        (set `local.RightLeftScale` 1.0)
        (elif (and (not (`self.KeyDPressing`)) (`self.KeyAPressing`))
          (set `local.RightLeftScale` -1.0)
          (else
            (set `local.RightLeftScale` 0.0)))))
    (:`then_2`
      (`/Game/Blueprints/MyBaseCharacter.UpdateMovementState` (`self.PlayerCharacter`) (`KismetMathLibrary.MakeVector2D` (`local.ForwardBackwardScale`) (`local.RightLeftScale`))))))

(fn `UserConstructionScript`)